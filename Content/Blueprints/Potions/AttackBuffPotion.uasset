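; Attack buff potion Blueprint that temporarily raises the player character's attack damage, ability power and true damage.
; UsePotion, gated by CanUsePotion, calls BuffDamage on player 0's BaseCharacter, waits out the effect duration, then calls DebuffDamage with the same amounts to revert it.
; PotionCooldown then waits the cooldown before re-enabling use, so the cooldown starts only after the effect ends.
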(event `self.UsePotion`
  (bind _asbase_character (cast `BaseCharacter` (`GameplayStatics.GetPlayerCharacter` 0) :!pure true))
  (if (`self.bCanUsePotion`)
    (`BaseCharacter.BuffDamage` _asbase_character (`self.AD_Buff`) (`self.AP_Buff`) (`self.TD_Buff`))
    (set `self.bCanUsePotion` false)
    (`KismetSystemLibrary.Delay` (`self.EffectDuration`))
    (`BaseCharacter.DebuffDamage` _asbase_character (`self.AD_Buff`) (`self.AP_Buff`) (`self.TD_Buff`))
    (`self.PotionCooldown`)))

(event `PotionCooldown`
  (`KismetSystemLibrary.Delay` (`self.Cooldown`))
  (set `self.bCanUsePotion` true))

(fn `UserConstructionScript`)