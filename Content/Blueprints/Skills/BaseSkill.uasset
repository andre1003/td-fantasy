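; Base skill actor that defines a player skill's damage, health and mana costs, cooldown and effect duration.
; On overlap, Shot-type skills add their attack, ability and true damage to the player's and call TakeHit on the enemy.
; GetDamage and GetCost return updated stats if the cost is affordable, otherwise unchanged values with zero cooldown.
; Movement and collision toggle functions are empty stubs.
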(event `self.ReceiveActorBeginOverlap`
  (params (OtherActor :type "Actor Object Reference"))
  (bind (_attackdamage _abilitypower _truedamage) (`/Game/TopDown/Blueprints/BP_TopDownCharacter.GetDamage` (cast `/Game/TopDown/Blueprints/BP_TopDownCharacter` (`GameplayStatics.GetPlayerCharacter` 0) :!pure true)))
  (switch `/Game/Data/Enum/SkillTypes` (`self.SkillType`)
    (:`NewEnumerator0`
      (bind _asbase_enemy (cast `/Game/Blueprints/Enemies/BP_BaseEnemy` OtherActor))
      (`/Game/Blueprints/Enemies/BP_BaseEnemy.TakeHit` _asbase_enemy (+ _attackdamage (`self.AttackDamage`)) (+ _abilitypower (`self.AbilityPower`)) (+ _truedamage (`self.TrueDamage`))))))

(fn `DisableCollision`)

(fn `EnableCollision`)

(fn `GetCost`
  (params (UserHealth :type Integer) (UserMana :type Integer))
  (returns (FinalHealth :type Integer) (FinalMana :type Integer) (Cooldown :type "Float (double-precision)"))
  (bind _returnvalue (- (`local.UserMana`) (`self.ManaCost`)))
  (bind _returnvalue_2 (- (`local.UserHealth`) (`self.HealthCost`)))
  (if (and (>= _returnvalue_2 0) (>= _returnvalue 0))
    (return _returnvalue_2 _returnvalue (`self.Cooldown`))
    (else
      (return (`local.UserHealth`) (`local.UserMana`) 0.0))))

(fn `GetDamage`
  (params (UserHealth :type Integer) (UserMana :type Integer) (UserAttackDamage :type Integer) (UserAbilityPower :type Integer) (UserTrueDamage :type Integer))
  (returns (FinalAttackDamage :type Integer) (FinalAbilityPower :type Integer) (FinalTrueDamage :type Integer) (FinalHealth :type Integer) (FinalMana :type Integer) (Cooldown :type "Float (double-precision)") (EffectDuration :type "Float (double-precision)") (SpawnOption :type "/Game/Data/Enum/SkillSpawnOptions Enum"))
  (if (and (>= (`local.UserHealth`) (`self.HealthCost`)) (>= (`local.UserMana`) (`self.ManaCost`)))
    (return (+ (`local.UserAttackDamage`) (`self.AttackDamage`)) (+ (`local.UserAbilityPower`) (`self.AbilityPower`)) (+ (`local.UserTrueDamage`) (`self.TrueDamage`)) (- (`local.UserHealth`) (`self.HealthCost`)) (- (`local.UserMana`) (`self.ManaCost`)) (`self.Cooldown`) (`self.EffectDuration`) (`self.SpawnOption`))
    (else
      (return (`local.UserAttackDamage`) (`local.UserAbilityPower`) (`local.UserTrueDamage`) (`local.UserHealth`) (`local.UserMana`) 0.0 0.0 "NewEnumerator0"))))

(fn `StartMovement`)

(fn `UserConstructionScript`)