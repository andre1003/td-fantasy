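; Player leveling system that tracks XP, level and attribute points, with popup widgets for XP gains and level-ups.
; AddXP triggers at most one LevelUp per call, which grants a point, boosts the top-down character's base stats, raises the XP threshold and refreshes the HUD.
; Per-level stat increments shrink at two milestone levels.
; LevelUpAttribute adds points to a chosen attribute after checking AvailablePoints, without deducting them.
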(fn `AddXP`
  (params (AddedXP :type Integer))
  (bind _output_get (set `self.XP` (+ AddedXP (`self.XP`))))
  (`self.DisplayAddXP_UI` AddedXP)
  (if (>= _output_get (`self.NextLevelXP`))
    (`self.LevelUp`)))

(fn `CalculateNextLevelXP`
  (set `self.NextLevelXP` (+ (`self.NextLevelXP`) (* (`self.BaseNextLevelXP`) (`self.Level`) 5))))

(fn `DisplayAddXP_UI`
  (params (AddedXP :type Integer))
  (bind _returnvalue (`|CreateWidget` "/Game/UI/Level/AddXPUI.AddXPUI_C"))
  (`/Game/UI/Level/AddXPUI.SetXPText` _returnvalue AddedXP)
  (`UserWidget.AddToViewport` _returnvalue 0))

(fn `DisplayLevelUpUI`
  (bind _returnvalue (`|CreateWidget` "/Game/UI/Level/LevelUpUI.LevelUpUI_C"))
  (`UserWidget.AddToViewport` _returnvalue 0))

(fn `IncreaseCD_AndUpgrade`
  (bind _level (`self.Level`))
  (if (== _level 40)
    (set `self.CooldownUpgrade` (- (`self.CooldownUpgrade`) 0.0001))
    (set `self.AttackSpeedUpgrade` (- (`self.AttackSpeedUpgrade`) 0.002))
    (elif (== _level 60)
      (set `self.CooldownUpgrade` (- (`self.CooldownUpgrade`) 0.00025))
      (set `self.AttackSpeedUpgrade` (- (`self.AttackSpeedUpgrade`) 0.003)))))

(fn `IncreaseDamageUpgrade`
  (bind _level (`self.Level`))
  (if (== _level 40)
    (set `self.DamageUpgrade` (- (`self.DamageUpgrade`) 2))
    (elif (== _level 60)
      (set `self.DamageUpgrade` (- (`self.DamageUpgrade`) 3)))))

(fn `IncreaseStatsUpgrade`
  (bind _level (`self.Level`))
  (if (== _level 40)
    (set `self.StatsUpgrade` (- (`self.StatsUpgrade`) 2))
    (elif (== _level 60)
      (set `self.StatsUpgrade` (- (`self.StatsUpgrade`) 3)))))

(fn `LevelUp`
  (set `self.XP` (- (`self.XP`) (`self.NextLevelXP`)))
  (if (< (`self.Level`) (`self.MaxLevel`))
    (`/Engine/EditorBlueprintResources/StandardMacros.IncrementInt` (`self.Level`)
      (:`  `
        (`/Engine/EditorBlueprintResources/StandardMacros.IncrementInt` (`self.AvailablePoints`)
          (:`  `
            (`self.DisplayLevelUpUI`)
            (`self.PassiveUpgrade`)
            (`self.CalculateNextLevelXP`)
            (`self.IncreaseStatsUpgrade`)
            (`self.IncreaseDamageUpgrade`)
            (`self.IncreaseCD_AndUpgrade`)
            (`self.UpdateHUD`)))))))

(fn `LevelUpAttribute`
  (params (PointsToUpgrade :type Integer) (Atribute :type "/Game/Data/Enum/PlayerAttributes Enum" :default "NewEnumerator0"))
  (if (>= (`self.AvailablePoints`) (`local.PointsToUpgrade`))
    (switch `/Game/Data/Enum/PlayerAttributes` Atribute
      (:`NewEnumerator0`
        (set `self.Life` (+ (`self.Life`) (`local.PointsToUpgrade`))))
      (:`NewEnumerator1`
        (set `self.Mana` (+ (`self.Mana`) (`local.PointsToUpgrade`))))
      (:`NewEnumerator2`
        (set `self.Endurance` (+ (`self.Endurance`) (`local.PointsToUpgrade`))))
      (:`NewEnumerator3`
        (set `self.Strength` (+ (`self.Strength`) (`local.PointsToUpgrade`))))
      (:`NewEnumerator4`
        (set `self.Dexterity` (+ (`self.Dexterity`) (`local.PointsToUpgrade`))))
      (:`NewEnumerator5`
        (set `self.Inteligence` (+ (`self.Inteligence`) (`local.PointsToUpgrade`))))
      (:`NewEnumerator6`
        (set `self.Arcane` (+ (`self.Arcane`) (`local.PointsToUpgrade`)))))))

(fn `PassiveUpgrade`
  (bind _asbp_top_down_character (cast `/Game/TopDown/Blueprints/BP_TopDownCharacter` (`GameplayStatics.GetPlayerCharacter` 0) :!pure true))
  (bind (_basehealth _basemana _baseattackdamage _baseabilitypower _basetruedamage _basebasicattackcooldown _baseattackspeed) (`/Game/TopDown/Blueprints/BP_TopDownCharacter.GetBaseStats` _asbp_top_down_character))
  (`/Game/TopDown/Blueprints/BP_TopDownCharacter.PassiveUpgrade` _asbp_top_down_character (+ _basehealth (`self.StatsUpgrade`)) (+ _basemana (`self.StatsUpgrade`)) (+ _baseattackdamage (`self.DamageUpgrade`)) (+ _baseabilitypower (`self.DamageUpgrade`)) (+ _basetruedamage (/ (`self.DamageUpgrade`) 3)) (- _basebasicattackcooldown (`self.CooldownUpgrade`)) (+ _baseattackspeed (`self.AttackSpeedUpgrade`))))

(fn `UpdateHUD`
  (bind _foundwidgets (`WidgetBlueprintLibrary.GetAllWidgetsOfClass` "/Game/UI/HUD.HUD_C"))
  (`/Game/UI/HUD.Update Stats Bar Size` (`|GetArrayItem` _foundwidgets)))

(fn `UserConstructionScript`)