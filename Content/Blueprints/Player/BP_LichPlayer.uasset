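; Lich player character Blueprint that adds a nearest-enemy search to its parent class.
; GetClosestEnemy spawns a temporary sphere component of the given range, picks the nearest living BaseEnemy overlapping it, then destroys the sphere.
; It stores the enemy, its location and a found flag in variables, falling back to the player's own location when none qualifies.
; Tick calls the parent and prints the DamageSystem poison status as debug output.
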(event `self.ReceiveTick`
  (params (DeltaSeconds :type "Float (single-precision)"))
  (`parent.ReceiveTick` DeltaSeconds)
  (`KismetSystemLibrary.PrintString` (`KismetStringLibrary.Concat_StrStr` "Poison status: " (`KismetStringLibrary.Conv_IntToString` (`DamageSystem.PoisonStatus` (`self.DamageSystem`)))) true true (struct :`R` 0.031152 :`G` 0.322917 :`A` 1.0) 0.0))

(event `self.GetClosestEnemy`
  (params (Range :type "Float (single-precision)"))
  (bind _index (`self.Index`))
  (set `self.Index` -1)
  (set `self.MinDistance` 5000000000.0)
  (set `self.ClosestEnemyTargetLocation` (0.0 0.0 0.0))
  (set `self.bEnemyWasFound` false)
  (set `self.EnemyFound` null)
  (bind _returnvalue (`AddComponent|NODE_AddSphereComponent-0`))
  (`SphereComponent.SetSphereRadius` _returnvalue Range true)
  (bind _overlappingactors (`PrimitiveComponent.GetOverlappingActors` _returnvalue "/Script/TDFantasyCpp.BaseEnemy"))
  (if (> (`KismetArrayLibrary.Array_Length` _overlappingactors) 0)
    (for (_array_element _array_index) _overlappingactors
      (bind _returnvalue_2 (`KismetMathLibrary.Vector_Distance` (`self.K2_GetActorLocation` _array_element) (`self.K2_GetActorLocation`)))
      (if (and (< _returnvalue_2 (`self.MinDistance`)) (not (`BaseEnemy.bIsDead` (cast `BaseEnemy` _array_element :!pure true))))
        (set `self.MinDistance` _returnvalue_2)
        (set `self.Index` _array_index)))
    (if (!= _index -1)
      (bind _output (`|GetArrayItem` _overlappingactors _index))
      (set `self.ClosestEnemyTargetLocation` (`self.K2_GetActorLocation` _output))
      (set `self.EnemyFound` (cast `BaseEnemy` _output :!pure true))
      (set `self.bEnemyWasFound` true)
      (`ActorComponent.K2_DestroyComponent` _returnvalue)
      (else
        (`ActorComponent.K2_DestroyComponent` _returnvalue)
        (set `self.ClosestEnemyTargetLocation` (`self.K2_GetActorLocation`))
        (set `self.EnemyFound` null)
        (set `self.bEnemyWasFound` false)))
    (else
      (`ActorComponent.K2_DestroyComponent` _returnvalue)
      (set `self.ClosestEnemyTargetLocation` (`self.K2_GetActorLocation`))
      (set `self.EnemyFound` null)
      (set `self.bEnemyWasFound` false))))

(fn `UserConstructionScript`)