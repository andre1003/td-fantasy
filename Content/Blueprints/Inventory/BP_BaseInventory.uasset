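; BP_BaseInventory is a base inventory Blueprint with pickup UI feedback and a slot-matching helper.
; AddUI creates a PickItemUI widget, fills it with the given amount plus the name and icon read from AddedItem's class defaults, then adds it to the viewport.
; HasItemOnSlot reports whether a valid slot holds a given item, returning false for invalid slots.
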(event `self.AddUI`
  (params (Amount :type Integer))
  (bind (_buyprice _sellprice _discoveryxp _itemtype _itemrarity _itemname _itemdescription _itemicon) (defaults `Object` (`self.AddedItem`)))
  (bind _returnvalue (`|CreateWidget` "/Game/UI/Inventory/PickItemUI.PickItemUI_C"))
  (`/Game/UI/Inventory/PickItemUI.SetItemInfo` _returnvalue Amount _itemname _itemicon)
  (`UserWidget.AddToViewport` _returnvalue 0))

(fn `HasItemOnSlot`
  (params (Slot :type "BaseInventorySlot Object Reference") (OtherItem :type "BaseItem Class Reference"))
  (returns (ReturnValue :type Boolean))
  (`/Engine/EditorBlueprintResources/StandardMacros.IsValid` Slot
    (:`Is Valid`
      (return (== (`BaseInventorySlot.Item` Slot) OtherItem)))
    (:`Is Not Valid`
      (return false))))

(fn `UserConstructionScript`)