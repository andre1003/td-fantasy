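; Inventory slot actor that holds one item reference, its amount and an empty flag.
; Add fills the slot and marks it occupied, while IncreaseAmount and DecreaseAmount adjust the stored count.
; When the count drops to zero or below, Remove looks up the Inventory actor by class, takes itself out of its Slots collection and destroys itself.
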(fn `Add`
  (params (ItemReference :type "/Game/Blueprints/Items/BaseItem Class Reference") (ItemAmount :type Integer))
  (set `self.Item` ItemReference)
  (set `self.Amount` ItemAmount)
  (set `self.IsEmpty` false))

(fn `DecreaseAmount`
  (params (AmountToDecrease :type Integer :default 1))
  (bind _output_get (set `self.Amount` (- (`self.Amount`) AmountToDecrease)))
  (if (<= _output_get 0)
    (`self.Remove`)))

(fn `IncreaseAmount`
  (params (AmountToAdd :type Integer))
  (set `self.Amount` (+ AmountToAdd (`self.Amount`))))

(fn `Remove`
  (bind _returnvalue (`GameplayStatics.GetActorOfClass` "/Game/Blueprints/Inventory/Inventory.Inventory_C"))
  (`KismetArrayLibrary.Array_RemoveItem` (`/Game/Blueprints/Inventory/Inventory.Slots` _returnvalue) self)
  (`self.K2_DestroyActor`))

(fn `UserConstructionScript`)