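; Inventory actor that tracks collected items as an array of Slot actors, each holding an item class and amount.
; AddItem shows a PickItemUI pickup widget using the item's class-default name and icon, then increases the matching slot or spawns and attaches a new one.
; HasItem searches slots linearly by class.
; RemoveItem decreases a matching slot's amount without removing it from the array itself.
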(fn `AddItem`
  (params (NewItem :type "/Game/Blueprints/Items/BaseItem Class Reference") (Amount :type Integer :default 1))
  (bind (_hasitem _itemslot) (`self.HasItem` NewItem))
  (`self.AddUI` NewItem Amount)
  (if _hasitem
    (`/Game/Blueprints/Inventory/Slot.IncreaseAmount` _itemslot Amount)
    (else
      (bind _returnvalue (`|SpawnActorFromClass` "/Game/Blueprints/Inventory/Slot.Slot_C" (`KismetMathLibrary.MakeTransform` (0.0 0.0 0.0)) "Undefined" "OverrideRootScale" null null))
      (`/Game/Blueprints/Inventory/Slot.Add` _returnvalue NewItem Amount)
      (`self.K2_AttachToActor` _returnvalue self "None" "KeepRelative" "KeepRelative" "KeepRelative" true)
      (`KismetArrayLibrary.Array_Add` (`self.Slots`) _returnvalue))))

(fn `AddUI`
  (params (ItemClassReference :type "/Game/Blueprints/Items/BaseItem Class Reference") (Amount :type Integer))
  (bind (_buyprice _sellprice _discoveryexperience _type _rarity _name _description _icon) (defaults `Object` ItemClassReference))
  (bind _returnvalue (`|CreateWidget` "/Game/UI/Inventory/PickItemUI.PickItemUI_C"))
  (`/Game/UI/Inventory/PickItemUI.SetItemInfo` _returnvalue Amount _name _icon)
  (`UserWidget.AddToViewport` _returnvalue 0))

(fn `HasItem`
  (params (ItemClass :type "/Game/Blueprints/Items/BaseItem Class Reference"))
  (returns (HasItem :type Boolean) (ItemSlot :type "/Game/Blueprints/Inventory/Slot Object Reference"))
  (bind _slots (`self.Slots`))
  (for (_array_element _array_index) _slots
    (if (== (`/Game/Blueprints/Inventory/Slot.Item` _array_element) ItemClass)
      (return true (`|GetArrayItem` _slots _array_index))))
  (return false null))

(fn `RemoveItem`
  (params (ItemToRemove :type "/Game/Blueprints/Items/BaseItem Class Reference") (Amount :type Integer :default 1))
  (bind (_hasitem _itemslot) (`self.HasItem` ItemToRemove))
  (if _hasitem
    (`/Game/Blueprints/Inventory/Slot.DecreaseAmount` _itemslot Amount)))

(fn `UserConstructionScript`)