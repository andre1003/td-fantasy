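; Base enemy character that patrols random nearby points and chases the player on sight via PawnSensing.
; Reaching the player triggers StartAttack, defined outside these graphs, with a cooldown re-attacking while the player stays visible and close.
; Rage swaps material and scales walk speed, while timelines drive slowdown recovery, damage flash and death fade through dynamic materials.
; CallFriends spawns a temporary sphere to make overlapping enemies join the chase.
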(event `self.SetupUI`
  ;[0 0 0] Health UI setup
  (bind _asenemy_health (cast `/Game/UI/EnemyHealth` (`WidgetComponent.GetWidget` (`self.HealthUI`))))
  (set `/Game/UI/EnemyHealth.Enemy` self _asenemy_health))

(event `self.ClearVisualEffect`
  (params (Effect :type "ParticleSystemComponent Object Reference") (LifeSpan :type "Float (single-precision)"))
  ;[0 0 0] Clear visual effect
  (`KismetSystemLibrary.Delay` LifeSpan)
  (`ActorComponent.Deactivate` Effect)
  (`KismetSystemLibrary.Delay` 1.0)
  (`ActorComponent.K2_DestroyComponent` Effect))

(event `self.RageEffect`
  (bind _charactermovement (`self.CharacterMovement`))
  (bind _mesh (`self.Mesh`))
  (bind _maxwalkspeed (`CharacterMovementComponent.MaxWalkSpeed` _charactermovement))
  ;[0 0 0] Rage effect setup
  (if (`self.bIsAngry`)
    (`PrimitiveComponent.SetMaterial` _mesh 1 (`self.RageMaterial`))
    (set `CharacterMovementComponent.MaxWalkSpeed` (* _maxwalkspeed 1.5) _charactermovement)
    (else
      (`PrimitiveComponent.SetMaterial` _mesh 1 (`self.NormalMaterial`))
      (set `CharacterMovementComponent.MaxWalkSpeed` (/ _maxwalkspeed 1.5) _charactermovement))))

(event `self.ClearTempDamage`
  ;[0 0 0] Reset temporary damage
  (`KismetSystemLibrary.RetriggerableDelay` 5.0)
  (set `self.TempDamageSuffered` 0))

(event `self.Patrol`
  ;[0 0 0] Enemy patrol
  (`KismetSystemLibrary.Delay` (`KismetMathLibrary.RandomFloatInRange` 2.0 5.0))
  (`|AIMoveTo` self (`NavigationSystemV1.K2_GetRandomReachablePointInRadius` (`self.K2_GetActorLocation`) 500.0 null null) null))

(event `self.PawnSensing.OnSeePawn`
  (params (Pawn :type "Pawn Object Reference"))
  ;[0 0 0] Combat
  (if (and (not (`self.bIsDead`)) (not (`BaseCharacter.bIsDead` (cast `BaseCharacter` (`self.PlayerReference`) :!pure true))))
    (cast `BaseCharacter` Pawn)
    (`self.ChasePlayer`)))

(event `self.ChasePlayer`
  ;[0 0 0] Combat
  (set `self.bCanSeeEnemy` true)
  (`|AIMoveTo` self (0.0 0.0 0.0) (`self.PlayerReference`) 75.0
    (:`OnSuccess`
      (`self.StartAttack`))))

(event `self.SlowDown`
  (bind _charactermovement (`self.CharacterMovement`))
  (bind _charactermovement_2 (`self.CharacterMovement`))
  ;[0 0 0] Combat
  (bind (_direction _speed) (`Timeline|SlowDownTimeline` :!via `PlayFromStart`)
    (:`Update`
      (if (`self.bIsAngry`)
        (set `CharacterMovementComponent.MaxWalkSpeed` (* _speed 1.5) _charactermovement)
        (else
          (set `CharacterMovementComponent.MaxWalkSpeed` _speed _charactermovement))))
    (:`Finished`
      (`KismetSystemLibrary.Delay` 0.2)
      (bind (_direction_2 _speed_2) (`Timeline|SpeedUpTimeline` :!via `PlayFromStart`)
        (:`Update`
          (if (`self.bIsAngry`)
            (set `CharacterMovementComponent.MaxWalkSpeed` (* _speed_2 1.5) _charactermovement_2)
            (else
              (set `CharacterMovementComponent.MaxWalkSpeed` _speed_2 _charactermovement_2))))))))

(event `self.DamageEffect`
  (bind _mesh (`self.Mesh`))
  ;[0 0 0] Combat
  (bind (_direction _damageeffect) (`Timeline|IncreaseDamageEffectTimeline` :!via `PlayFromStart`)
    (:`Update`
      (bind _returnvalue (`PrimitiveComponent.CreateDynamicMaterialInstance` _mesh 1 (`PrimitiveComponent.GetMaterial` _mesh 1) "None"))
      (`MaterialInstanceDynamic.SetScalarParameterValue` _returnvalue "DamageEffectAlpha" _damageeffect))
    (:`Finished`
      (`KismetSystemLibrary.Delay` 0.05)
      (bind (_direction_2 _damageeffect_2) (`Timeline|DecreaseDamageEffectTimeline` :!via `PlayFromStart`)
        (:`Update`
          (`MaterialInstanceDynamic.SetScalarParameterValue` _returnvalue "DamageEffectAlpha" _damageeffect_2))))))

(event `self.StartAttackCooldown`
  ;[0 0 0] Combat
  (`KismetSystemLibrary.Delay` (`self.AttackCooldown`))
  (set `self.AttackCooldown` 0.0)
  (if (and (`self.bCanSeeEnemy`) (< (`KismetMathLibrary.Vector_Distance` (`self.K2_GetActorLocation`) (`self.K2_GetActorLocation` (`self.PlayerReference`))) 200.0) (not (`self.bIsDead`)))
    (`self.StartAttack`)
    (else
      (set `self.bIsAttacking` false))))

(event `self.DeathEffect`
  (bind _mesh (`self.Mesh`))
  ;[0 0 0] Combat
  (bind (_direction _opacity) (`Timeline|DeathEffectTimeline` :!via `PlayFromStart`)
    (:`Update`
      (for _index (range (`PrimitiveComponent.GetNumMaterials` _mesh))
        (bind _returnvalue (`PrimitiveComponent.CreateDynamicMaterialInstance` _mesh _index (`PrimitiveComponent.GetMaterial` _mesh _index) "None"))
        (`MaterialInstanceDynamic.SetScalarParameterValue` _returnvalue "Opacity" _opacity)))))

(event `self.CallFriends`
  ;[0 0 0] Combat
  (if (not (`self.bIsDead`))
    (bind _returnvalue (`|AddComponentByClass` "/Script/Engine.SphereComponent" false (`KismetMathLibrary.MakeTransform` (0.0 0.0 0.0))))
    (`SphereComponent.SetSphereRadius` _returnvalue (`self.CallFriendsRange`) true)
    (for _array_element (`PrimitiveComponent.GetOverlappingActors` _returnvalue "/Script/TDFantasyCpp.BaseEnemy")
      (`self.ChasePlayer` (cast `BaseEnemy` _array_element :!pure true)))
    (`ActorComponent.K2_DestroyComponent` _returnvalue)))

(fn `StopChasePlayer`
  (returns (ReturnValue :type Boolean))
  (bind _playerreference (`self.PlayerReference`))
  (return (or (> (`KismetMathLibrary.Vector_Distance` (`self.K2_GetActorLocation`) (`self.K2_GetActorLocation` _playerreference)) (`self.MaxDistanceFromEnemy`)) (`BaseCharacter.bIsDead` (cast `BaseCharacter` _playerreference :!pure true)))))

(fn `UserConstructionScript`)