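; Dialog component that runs a conversation through a Behavior Tree when a player character interacts.
; It spawns its own DialogAIController at BeginPlay solely to host the dialog tree and blackboard.
; On interaction it shows a DialogUI widget, switches the player controller's mode, starts the tree and passes the widget in through the blackboard.
; The widget's exit event switches the mode again, stops the tree logic and removes the widget.
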(event `self.ReceiveBeginPlay`
  (bind _returnvalue (`|SpawnActorFromClass` "/Game/Blueprints/DialogSystem/DialogAIController.DialogAIController_C" (`KismetMathLibrary.MakeTransform` (0.0 0.0 0.0)) "Undefined" "OverrideRootScale" null null))
  (set `self.AIController` _returnvalue))

(event `/Game/Blueprints/DialogSystem/InteractionInterface.OnInteraction`
  (params (PlayerCharacter :type "BaseCharacter Object Reference"))
  (bind _output_get (set `self.PlayerController` (cast `/Game/Blueprints/PlayerController/BP_TDFPlayerController` (`Pawn.GetController` PlayerCharacter) :!pure true)))
  (bind _returnvalue (`|CreateWidget` "/Game/UI/Dialog/DialogUI.DialogUI_C" _output_get))
  (bind _output_get_2 (set `self.DialogWidget` _returnvalue))
  (add `/Game/UI/Dialog/DialogUI.OnExit` _output_get_2 (delegate `OnExit`))
  (`UserWidget.AddToViewport` _output_get_2 0)
  (`TDFPlayerController.ChangeMode` _output_get 1)
  (`AIController.RunBehaviorTree` (`self.AIController`) (`self.DialogTree`))
  (bind _blackboardcomponent (`AIController.UseBlackboard` (`self.AIController`) "/Game/Blueprints/DialogSystem/DialogBlackboard.DialogBlackboard"))
  (`BlackboardComponent.SetValueAsObject` _blackboardcomponent "DialogWidget" (`self.DialogWidget`)))

(event `OnExit`
  (`TDFPlayerController.ChangeMode` (`self.PlayerController`) 2)
  (`BrainComponent.StopLogic` (`AIController.BrainComponent` (`self.AIController`)) "Dialog Exited")
  (`Widget.RemoveFromParent` (`self.DialogWidget`)))