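; Base lootable chest that the player opens to receive items, random coins and gems, and XP.
; Overlap registers it as the top-down character's TempChest while closed and shows an "Open" widget, cleared on exit.
; OpenChest runs CollectItems before its IsOpen check, feeding the Inventory actor and player, then swings the lid via chained timelines with a hit-back.
; CollectItems removes array entries while iterating them; location and yaw timelines are unused.
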(event `self.ReceiveBeginPlay`
  (`self.SetUseText` (`.AsUse UI` (cast `` (`WidgetComponent.GetWidget` (`self.UseUI`)) :!pure true)) "Open"))

(event `self.ReceiveActorBeginOverlap`
  (params (OtherActor :type "Actor Object Reference"))
  (bind _useui (`self.UseUI`))
  (if (not (`self.IsOpen`))
    (bind _asbp_top_down_character (cast `/Game/TopDown/Blueprints/BP_TopDownCharacter` OtherActor))
    (set `/Game/TopDown/Blueprints/BP_TopDownCharacter.TempChest` self _asbp_top_down_character)
    (`SceneComponent.SetVisibility` _useui true false)
    (`self.ShowUI` (`.AsUse UI` (cast `` (`WidgetComponent.GetWidget` _useui) :!pure true)))))

(event `self.ReceiveActorEndOverlap`
  (params (OtherActor :type "Actor Object Reference"))
  (bind _useui (`self.UseUI`))
  (bind _asbp_top_down_character (cast `/Game/TopDown/Blueprints/BP_TopDownCharacter` OtherActor))
  (set `/Game/TopDown/Blueprints/BP_TopDownCharacter.TempChest` null _asbp_top_down_character)
  (`self.HideUI` (`.AsUse UI` (cast `` (`WidgetComponent.GetWidget` _useui) :!pure true)))
  (`KismetSystemLibrary.Delay` 0.25)
  (`SceneComponent.SetVisibility` _useui false false))

(event `OpenChest`
  (bind _superior (`self.Superior`))
  (`SceneComponent.SetVisibility` (`self.UseUI`) false false)
  (`self.CollectItems`)
  (if (not (`self.IsOpen`))
    (`|ExecutionSequence`
      (:`then_0`
        (bind (_direction _xrotation) (`Timeline|XRotationTimeline` :!via `PlayFromStart`)
          (:`Update`
            (`SceneComponent.K2_SetRelativeRotation` _superior (`KismetMathLibrary.MakeRotator` _xrotation) false false))
          (:`Finished`
            (bind (_direction_2 _xrotation_2) (`Timeline|XRotationHitBackTimeline` :!via `PlayFromStart`)
              (:`Update`
                (`SceneComponent.K2_SetRelativeRotation` _superior (`KismetMathLibrary.MakeRotator` _xrotation_2) false false))))))
      (:`then_2`
        (set `self.IsOpen` true)))))

(fn `CollectItems`
  (bind _items (`self.Items`))
  (bind _asbp_top_down_character (cast `/Game/TopDown/Blueprints/BP_TopDownCharacter` (`GameplayStatics.GetPlayerCharacter` 0) :!pure true))
  (bind _returnvalue (`GameplayStatics.GetActorOfClass` "/Game/Blueprints/Inventory/Inventory.Inventory_C"))
  (for (_array_element _array_index) _items
    (`/Game/Blueprints/Inventory/Inventory.AddItem` _returnvalue _array_element (`|GetArrayItem` (`self.ItemsAmount`) _array_index))
    (`KismetArrayLibrary.Array_Remove` _items _array_index)
    (`KismetArrayLibrary.Array_Remove` (`self.ItemsAmount`) _array_index))
  (`/Game/TopDown/Blueprints/BP_TopDownCharacter.AddMoney` _asbp_top_down_character (`KismetMathLibrary.RandomIntegerInRange` 0 (`self.MaxCoins`)) (`KismetMathLibrary.RandomIntegerInRange` 0 (`self.MaxGems`)))
  (`/Game/Blueprints/Level/LevelSystem.AddXP` (`/Game/TopDown/Blueprints/BP_TopDownCharacter.Level` _asbp_top_down_character) (`self.XP`)))

(fn `UserConstructionScript`)