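; Base item actor that the top-down character can approach, showing a "Collect" prompt through a UseUI widget component.
; On overlap it registers itself as the character's TempItem, makes the widget visible and calls ShowUI.
; On end overlap it clears TempItem, calls HideUI and hides the component after a short delay.
; UseItem is an empty function, apparently a hook for child items to implement.
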(event `self.ReceiveBeginPlay`
  (`/Game/UI/UseUI.SetUseText` (cast `/Game/UI/UseUI` (`WidgetComponent.GetWidget` (`self.UseUI`)) :!pure true) "Collect"))

(event `self.ReceiveActorBeginOverlap`
  (params (OtherActor :type "Actor Object Reference"))
  (bind _useui (`self.UseUI`))
  (bind _asbp_top_down_character (cast `/Game/TopDown/Blueprints/BP_TopDownCharacter` OtherActor))
  (set `/Game/TopDown/Blueprints/BP_TopDownCharacter.TempItem` self _asbp_top_down_character)
  (`SceneComponent.SetVisibility` _useui true false)
  (bind _asuse_ui (cast `/Game/UI/UseUI` (`WidgetComponent.GetWidget` _useui)))
  (`/Game/UI/UseUI.ShowUI` _asuse_ui))

(event `self.ReceiveActorEndOverlap`
  (params (OtherActor :type "Actor Object Reference"))
  (bind _useui (`self.UseUI`))
  (bind _asbp_top_down_character (cast `/Game/TopDown/Blueprints/BP_TopDownCharacter` OtherActor))
  (set `/Game/TopDown/Blueprints/BP_TopDownCharacter.TempItem` null _asbp_top_down_character)
  (bind _asuse_ui (cast `/Game/UI/UseUI` (`WidgetComponent.GetWidget` _useui)))
  (`/Game/UI/UseUI.HideUI` _asuse_ui)
  (`KismetSystemLibrary.Delay` 0.25)
  (`SceneComponent.SetVisibility` _useui false false))

(fn `UseItem`)

(fn `UserConstructionScript`)