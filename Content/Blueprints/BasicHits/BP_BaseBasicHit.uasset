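; Base actor for the player's basic hit, which damages the first living BP_BaseEnemy it overlaps and then destroys itself.
; On spawn it sums the player's attack and true damage, passing the total to TakeHit as attack damage only.
; A replaying timeline flickers its point light, and a five-second lifespan limits it.
; Its MoveComponentTo targets the actor's own location, behind an always-true branch.
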(event `self.ReceiveBeginPlay`
  (`|ExecutionSequence`
    (:`then_0`
      (bind (_direction _intensity) (`Timeline|FlickingTimeline` :!via `PlayFromStart` :!label _label)
        (:`Update`
          (`LightComponent.SetIntensity` (`self.PointLight`) (* _intensity 200.0)))
        (:`Finished`
          (`KismetSystemLibrary.Delay` 1.0)
          (goto _label :!via `PlayFromStart`))))
    (:`then_1`
      (if true
        (`KismetSystemLibrary.MoveComponentTo` (`self.RootComponent`) (`self.K2_GetActorLocation` null))
        (else
          (`self.K2_DestroyActor`))))
    (:`then_2`
      (`self.CalculateDamage`))
    (:`then_3`
      (`self.SetLifeSpan` 5.0))))

(event `self.ReceiveActorBeginOverlap`
  (params (OtherActor :type "Actor Object Reference"))
  (bind _asbase_enemy (cast `/Game/Blueprints/Enemies/BP_BaseEnemy` OtherActor))
  (if (not (`/Game/Blueprints/Enemies/BP_BaseEnemy.GetIsDead` _asbase_enemy))
    (`/Game/Blueprints/Enemies/BP_BaseEnemy.TakeHit` _asbase_enemy (`self.Damage`) 0 0)
    (`self.K2_DestroyActor`)))

(fn `CalculateDamage`
  (bind _asbp_top_down_character (cast `/Game/TopDown/Blueprints/BP_TopDownCharacter` (`GameplayStatics.GetPlayerCharacter` 0) :!pure true))
  (set `self.Damage` (+ (`/Game/TopDown/Blueprints/BP_TopDownCharacter.AttackDamage` _asbp_top_down_character) (`/Game/TopDown/Blueprints/BP_TopDownCharacter.TrueDamage` _asbp_top_down_character))))

(fn `UserConstructionScript`)